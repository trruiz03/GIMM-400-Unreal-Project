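; LapTimer_GM, apparently a game mode, tracks lap progress and race completion.
; BeginPlay resets the completed lap count, sets the required count and builds the initial LapText.
; UpdateLaps refreshes that "completed/required" text through LapsAsText and sets RaceComplete once the target is reached.
; The lap count is never incremented here, and no timing logic is present.
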(event `self.ReceiveBeginPlay`
  (bind _output_get (set `self.LapsRequired` 2))
  (bind _output_get_2 (set `self.LapsCompleted` 0))
  (set `self.LapText` (`self.Laps As Text` _output_get_2 _output_get)))

(event `UpdateLaps`
  (bind _lapscompleted (`self.LapsCompleted`))
  (bind _lapsrequired (`self.LapsRequired`))
  (set `self.LapText` (`self.Laps As Text` _lapscompleted _lapsrequired))
  (if (>= _lapscompleted _lapsrequired)
    (set `self.RaceComplete` true)))

(fn `UserConstructionScript`)