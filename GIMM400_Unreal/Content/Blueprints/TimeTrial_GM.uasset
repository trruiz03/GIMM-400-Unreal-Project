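; Game mode for a time trial race that tracks lap progress and flags when the race is complete.
; BeginPlay sets the required lap count, resets completed laps and initializes the lap text.
; UpdateLaps refreshes that text through LapsAsText and sets RaceComplete once enough laps are done; the lap count is not incremented here.
; LapsAsText holds completed/required formatting nodes, shown as unused in its graph.
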(event `self.ReceiveBeginPlay`
  (bind _output_get (set `self.LapRequired` 2))
  (bind _output_get_2 (set `self.LapsCompleted` 0))
  (set `self.LapText` (`self.Laps As Text` _output_get_2 _output_get)))

(event `UpdateLaps`
  (bind _laprequired (`self.LapRequired`))
  (bind _lapscompleted (`self.LapsCompleted`))
  (set `self.LapText` (`self.Laps As Text` _lapscompleted _laprequired))
  (if (>= _lapscompleted _laprequired)
    (set `self.RaceComplete` true)))

(fn `UserConstructionScript`)