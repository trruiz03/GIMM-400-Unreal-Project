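; StartLine_BP is the start line trigger for a time trial vehicle race.
; On BeginPlay it caches the VehiclePlayerController and the TimeTrial_GM game mode.
; The first Box overlap starts a lap and, through a DoOnce, starts the race.
; Later overlaps increment the game mode's completed lap count, start a new lap and update laps, with no check on which actor overlapped.
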(event `self.ReceiveBeginPlay`
  (bind _asvehicle_player_controller (cast `/Game/VehicleTemplate/Blueprints/VehiclePlayerController` (`GameplayStatics.GetPlayerController` 0)))
  (set `self.As Vehicle Player Controller` _asvehicle_player_controller)
  (bind _astime_trial_gm (cast `/Game/Blueprints/TimeTrial_GM` (`GameplayStatics.GetGameMode`)))
  (set `self.As Time Trial GM` _astime_trial_gm))

(event `self.Box.OnComponentBeginOverlap`
  (params (OverlappedComponent :type "PrimitiveComponent Object Reference") (OtherActor :type "Actor Object Reference") (OtherComp :type "PrimitiveComponent Object Reference") (OtherBodyIndex :type Integer) (bFromSweep :type Boolean) (SweepResult :type "HitResult Structure (by ref)"))
  (bind _as_vehicle_player_controller (`self.As Vehicle Player Controller`))
  (bind _as_time_trial_gm (`self.As Time Trial GM`))
  (if (`self.RaceStarted`)
    (`/Engine/EditorBlueprintResources/StandardMacros.IncrementInt` (`/Game/Blueprints/TimeTrial_GM.LapsCompleted` _as_time_trial_gm)
      (:`  `
        (`/Game/VehicleTemplate/Blueprints/VehiclePlayerController.Start Lap` _as_vehicle_player_controller)
        (`/Game/Blueprints/TimeTrial_GM.UpdateLaps` _as_time_trial_gm)))
    (else
      (`/Game/VehicleTemplate/Blueprints/VehiclePlayerController.Start Lap` _as_vehicle_player_controller)
      (`/Engine/EditorBlueprintResources/StandardMacros.DoOnce` false
        (:`Completed`
          (`/Game/VehicleTemplate/Blueprints/VehiclePlayerController.Start Race` _as_vehicle_player_controller)
          (set `self.RaceStarted` true))))))

(fn `UserConstructionScript`)